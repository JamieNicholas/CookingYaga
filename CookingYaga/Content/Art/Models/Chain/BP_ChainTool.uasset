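; BP_ChainTool is a spline-based construction tool that lays out a chain of static mesh links in the level.
; The construction script divides the spline length by Spacing and adds two unattached mesh components per step, placed and rotated by world-space spline samples.
; The half-step links get an extra 90-degree roll, so neighbors alternate like interlocking chain links.
; The event graph holds only disabled stubs, so there is no runtime logic.
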(event EventBeginPlay)

(event Collision|EventActorBeginOverlap
  (params (OtherActor :type Actor%20Object%20Reference)))

(event EventTick
  (params (DeltaSeconds :type Float%20%28single-precision%29)))

(fn ConstructionScript
  (bind _spline (Variables|Default|GetSpline))
  (bind _spacing (Variables|Default|GetSpacing))
  (for _index (range 1 (.ReturnValue (Math|Float|Division(WholeandRemainder) (Spline|GetSplineLength _spline) _spacing)))
    (AddComponent|AddStaticMeshComponent true (Math|Transform|MakeTransform (Spline|GetLocationatDistanceAlongSpline _spline (* _index _spacing) "World") (Spline|GetRotationatDistanceAlongSpline _spline (* _index _spacing) "World")))
    (AddComponent|AddStaticMeshComponent true (Math|Transform|MakeTransform (Spline|GetLocationatDistanceAlongSpline _spline (- (* _index _spacing) (/ _spacing 2.0)) "World") (Math|Rotator|MakeRotator (+ (.Roll (Math|Rotator|BreakRotator (Spline|GetRotationatDistanceAlongSpline _spline (- (* _index _spacing) (/ _spacing 2.0)) "World"))) 9e+01) (.Pitch (Math|Rotator|BreakRotator (Spline|GetRotationatDistanceAlongSpline _spline (- (* _index _spacing) (/ _spacing 2.0)) "World"))) (.Yaw (Math|Rotator|BreakRotator (Spline|GetRotationatDistanceAlongSpline _spline (- (* _index _spacing) (/ _spacing 2.0)) "World"))))))))