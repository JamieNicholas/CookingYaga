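; ForestCross is a trigger Blueprint that switches the level's ambience and music to the forest set when its box is overlapped.
; On box overlap, a sequence first stops the forest, streams and desert ambient sounds, then restarts forest ambience.
; It then does the same for the three music tracks, restarting forest music from the beginning.
; The overlapping actor is not filtered, and a leftover PlaySound2D node is never run.
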(event OnComponentBeginOverlap(Box)
  (params (OverlappedComponent :type Primitive%20Component%20Object%20Reference) (OtherActor :type Actor%20Object%20Reference) (OtherComp :type Primitive%20Component%20Object%20Reference) (OtherBodyIndex :type Integer) (bFromSweep :type Boolean) (SweepResult :type Hit%20Result%20Structure%20%28by%20ref%29))
  (Utilities|FlowControl|Sequence
    (:then_0
      (Audio|Components|Audio|Stop (Variables|/Script/Engine.AmbientSound|GetAudioComponent (Variables|Default|GetForestSound)))
      (Audio|Components|Audio|Stop (Variables|/Script/Engine.AmbientSound|GetAudioComponent (Variables|Default|GetStreamsSound)))
      (Audio|Components|Audio|Stop (Variables|/Script/Engine.AmbientSound|GetAudioComponent (Variables|Default|GetDesertSound)))
      (Audio|Components|Audio|Play (Variables|/Script/Engine.AmbientSound|GetAudioComponent (Variables|Default|GetForestSound)) 0.0))
    (:then_1
      (Audio|Components|Audio|Stop (Variables|/Script/Engine.AmbientSound|GetAudioComponent (Variables|Default|GetForestMusic)))
      (Audio|Components|Audio|Stop (Variables|/Script/Engine.AmbientSound|GetAudioComponent (Variables|Default|GetStreamsMusc)))
      (Audio|Components|Audio|Stop (Variables|/Script/Engine.AmbientSound|GetAudioComponent (Variables|Default|GetDesertMusic)))
      (Audio|Components|Audio|Play (Variables|/Script/Engine.AmbientSound|GetAudioComponent (Variables|Default|GetForestMusic)) 0.0))))

(event EventBeginPlay)

(event Collision|EventActorBeginOverlap
  (params (OtherActor :type Actor%20Object%20Reference)))

(event EventTick
  (params (DeltaSeconds :type Float%20%28single-precision%29)))

(fn ConstructionScript)