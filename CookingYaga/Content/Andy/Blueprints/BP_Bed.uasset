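; BP_Bed is an interactable bed that ends the current in-game day.
; Interacting shows the UI_EndOfDay widget, initialized with the day number and potion tally, then calls DayReset, whose bound handler increments the day.
; Neworderfulfilled feeds that tally, looking up potion details in PotionManager and raising the per-potion quantity in the OrderMadePotions map.
; The file never clears the tally between days.
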(event Custom|TriggerSleep
  ;[1 1 1] TriggerSleep
  (bind _returnvalue (UserInterface|CreateWidget "/Game/Andy/UI/EndOfDay/UI_EndOfDay.UI_EndOfDay_C" (Game|GetPlayerController 0)))
  (bind _output_get (Variables|Default|SetEnd%20Of%20Day _returnvalue))
  (Default|Init _output_get (Variables|Default|GetOrder%20made%20potions) (Variables|Default|GetDay))
  (UserInterface|Viewport|AddtoViewport _returnvalue 0)
  (Default|CallDayReset))

(event Custom|New%20order%20fulfilled
  (params (Potion%20ID :type Integer))
  (bind _potion_manager (Variables|Default|GetPotion%20Manager))
  (bind _order_made_potions (Variables|Default|GetOrder%20made%20potions))
  (bind _potions (Variables|/Game/Rowan/Cooking_Yaga_Cauldron_etc/Blues/Potions/Potion_Manager.Potion_Manager_C|GetPotions _potion_manager))
  (bind _value (Utilities|Map|Find _potions Potion%20ID))
  (bind _potionid (Utilities|Struct|BreakPotion_details _value))
  (bind (_value_2 _returnvalue) (Utilities|Map|Find _order_made_potions _potionid))
  (if _returnvalue
    (Utilities|Map|Remove _order_made_potions _potionid)
    (Utilities|Map|Add _order_made_potions _potionid (Utilities|Struct|MakeEndofDay_Details (.potiondetails _value_2) (+ (.quantity _value_2) 1)))
    (else
      (Utilities|Map|Add _order_made_potions _potionid (Utilities|Struct|MakeEndofDay_Details _value 1)))))

(event Custom|Update%20Day
  ;[1 1 1] TriggerSleep
  (Math|Integer|IncrementInt (Variables|Default|GetDay)))

(event EventBeginPlay
  ;[1 1 1] TriggerSleep
  (EventDispatchers|BindEventtoDayReset (delegate Custom|Update%20Day)))

(event EventButtonInteract
  (params (IsCalled :type Boolean))
  (CallFunction|TriggerSleep))

(fn ConstructionScript)