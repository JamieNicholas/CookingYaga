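; BP_UgradesManager is a manager Blueprint meant to respond to upgrade changes for fabrics, lantern, sign, roof, temp and cauldron.
; On BeginPlay it binds one custom event to each of those change notifications.
; All handler events are currently empty, and the call to upgrade the referenced cauldron is disconnected, so the bindings have no effect yet.
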(event Custom|ChangeFabric)

(event Custom|ChangeLantern)

(event Custom|ChangeSign)

(event Custom|ChangeRoof)

(event Custom|ChangeTemp)

(event Custom|UpgradeCauldron)

(event EventBeginPlay
  (EventDispatchers|BindEventtoFabricsChanged (delegate Custom|ChangeFabric))
  (EventDispatchers|BindEventtoLanternChanged (delegate Custom|ChangeLantern))
  (EventDispatchers|BindEventtoSignChanged (delegate Custom|ChangeSign))
  (EventDispatchers|BindEventtoRoofChanged (delegate Custom|ChangeRoof))
  (EventDispatchers|BindEventtoTempChanged (delegate Custom|ChangeTemp))
  (EventDispatchers|BindEventtoCauldronUpgraded (delegate Custom|UpgradeCauldron)))

(fn ConstructionScript)