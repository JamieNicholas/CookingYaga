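; Small stove door that the player toggles open and closed through a button interaction, with a "Press E to open door" prompt.
; ButtonInteract calls TriggerDoor, which plays or reverses a timeline that lerps the Door's relative rotation between DoorRot and a fixed open angle.
; IsOpening blocks retriggering during the swing, and IsOpen flips when the timeline finishes.
; The ingredient and potion detail getters are empty.
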(event Custom|TriggerDoor
  ;[1 1 1] TriggerDoor
  (if (not (Variables|Default|GetIsOpening))
    (if (Variables|Default|GetIsOpen)
      (bind _dooropen (Timeline|Timeline_0 ReverseFromEnd)
        (:Update
          (Variables|Default|SetIsOpening true)
          (Transformation|SetRelativeRotation (Variables|Default|GetDoor) (Math|Rotator|Lerp(Rotator) (Variables|Default|GetDoorRot) "0,100.000000, 0" _dooropen true) false false))
        (:Finished
          (Variables|Default|SetIsOpen (not (Variables|Default|GetIsOpen)))
          (Variables|Default|SetIsOpening false)))
      (else
        (Timeline|Timeline_0 Play)))))

(event EventButtonInteract
  (params (IsCalled :type Boolean))
  (CallFunction|TriggerDoor))

(fn ConstructionScript)

(fn GetIngrediantDetails
  (return ""))

(fn GetMiscName
  (return "Press E to open door"))

(fn GetPotionDetails
  (return ""))