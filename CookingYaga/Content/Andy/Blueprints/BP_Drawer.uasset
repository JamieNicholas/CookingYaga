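; BP_Drawer is an interactable drawer that slides open and closed when the player triggers it, showing a "Press E to open" prompt.
; The construction script caches the drawer's starting location, and a timeline lerps it 30 units along relative Y from there, playing forward or in reverse.
; IsOpening blocks retriggers during motion, and IsOpen flips when the timeline finishes.
; The ingredient and potion detail getters are empty.
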(event Custom|TriggerDrawer
  ;[1 1 1] TriggerDrawer
  (if (not (Variables|Default|GetIsOpening))
    (if (Variables|Default|GetIsOpen)
      (bind _dooropen (Timeline|Timeline_0 ReverseFromEnd)
        (:Update
          (Variables|Default|SetIsOpening true)
          (Transformation|SetRelativeLocation (Variables|Default|GetDrawer) (Math|Vector|Lerp(Vector) (Variables|Default|GetDrawerLoc) (+ (Variables|Default|GetDrawerLoc) "0,30.000000, 0") _dooropen) false false))
        (:Finished
          (Variables|Default|SetIsOpen (not (Variables|Default|GetIsOpen)))
          (Variables|Default|SetIsOpening false)))
      (else
        (Timeline|Timeline_0 Play)))))

(event EventButtonInteract
  (params (IsCalled :type Boolean))
  (CallFunction|TriggerDrawer))

(fn ConstructionScript
  (Variables|Default|SetDrawerLoc (Variables|/Script/Engine.SceneComponent|GetRelativeLocation (Variables|Default|GetDrawer))))

(fn GetIngrediantDetails
  (return ""))

(fn GetMiscName
  (return "Press E to open"))

(fn GetPotionDetails
  (return ""))